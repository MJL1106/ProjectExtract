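; BP_Laser is a weapon attachment with an aiming laser and a toggleable flashlight.
; While active, it traces from the Laser socket every tick, placing the dot on the hit surface and stretching the beam by distance.
; Dot size scales with distance and viewport resolution through a material parameter collection, which also carries flashlight state.
; GetBulletTransform aims shots from the muzzle at the laser hit point, and a LaserActive RepNotify drives visibility.
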(event `self.ReceiveBeginPlay`
  (set `self.LaserActive` true))

(event `self.ReceiveTick`
  (params (DeltaSeconds :type "Float (single-precision)"))
  (`self.LaserDotTrace`))

(fn `GetBulletTransform`
  (params (MuzzleTransform :type "Transform Structure"))
  (returns (Output :type "Transform Structure"))
  (bind _location (.location MuzzleTransform))
  (return (select `bool` (`self.LaserActive`) :`false` (`KismetMathLibrary.MakeTransform` _location (.rotation MuzzleTransform)) :`true` (`KismetMathLibrary.MakeTransform` _location (`KismetMathLibrary.FindLookAtRotation` _location (`self.LaserHitLocation`))))))

(fn `LaserDotTrace`
  (bind (_returnvalue_x _returnvalue_y) (`KismetMathLibrary.BreakVector2D` (`WidgetLayoutLibrary.GetViewportSize`)))
  (bind _laserdot (`self.LaserDot`))
  (bind _returnvalue (`KismetMathLibrary.SelectFloat` 1.25 1.0 (`self.UseIRLaser`)))
  (bind (_returnvalue_location _returnvalue_rotation) (`KismetMathLibrary.BreakTransform` (`SceneComponent.GetSocketTransform` (`self.Mesh`) "Laser" "RTS_World")))
  (if (`self.LaserActive`)
    (bind (_outhit _returnvalue_2) (`KismetSystemLibrary.LineTraceSingle` _returnvalue_location (+ _returnvalue_location (* (`KismetMathLibrary.GetForwardVector` _returnvalue_rotation) 100000.0)) "TraceTypeQuery2" false (`|MakeArray` (`self.GetOwner`) (`GameplayStatics.GetPlayerPawn` 0) :!type "Actor Object Reference")))
    (`SceneComponent.SetVisibility` _laserdot _returnvalue_2 false)
    (if _returnvalue_2
      (bind (_bblockinghit _binitialoverlap _time _distance _location _impactpoint _normal _impactnormal _physmat _hitactor _hitcomponent _hitbonename _bonename _hititem _elementindex _faceindex _tracestart _traceend) (`GameplayStatics.BreakHitResult` _outhit))
      (bind _output_get (set `self.LaserHitLocation` _location))
      (`SceneComponent.K2_SetWorldLocationAndRotation` _laserdot _output_get (`KismetMathLibrary.MakeRotFromX` _normal) false false)
      (`SceneComponent.SetWorldScale3D` (`self.LaserBeam`) (`KismetMathLibrary.MakeVector` (/ _distance 20.0) _returnvalue _returnvalue))
      (`KismetMaterialLibrary.SetScalarParameterValue` "/Game/ProceduralFPSKIT/Blueprints/Attachments/Laser/Materials/MPC_LaserControls.MPC_LaserControls" "LaserDotSize" (`KismetMathLibrary.MapRangeClamped` (* (/ _distance (* _returnvalue_x _returnvalue_y)) 1000.0) 0.0 2.0 0.125 0.5))
      (else
        (set `self.LaserHitLocation` _traceend)))))

(fn `OnRep_LaserActive`
  (`SceneComponent.SetVisibility` (`self.LaserBeam`) (`self.LaserActive`) false)
  (`SceneComponent.SetVisibility` (`self.LaserDot`) (`self.LaserActive`) false))

(fn `ToggleFlashlight`
  (params (bNewVisibility :type Boolean))
  (`SceneComponent.SetVisibility` (`self.Flashlight`) bNewVisibility false)
  (`KismetMaterialLibrary.SetScalarParameterValue` "/Game/ProceduralFPSKIT/Blueprints/Attachments/Laser/Materials/MPC_LaserControls.MPC_LaserControls" "UseFlashlight" (`KismetMathLibrary.Conv_BoolToDouble` bNewVisibility)))

(fn `ToggleLaser`
  (params (`TurnOn?` :type Boolean))
  (set `self.LaserActive` `TurnOn?`))

(fn `UserConstructionScript`
  (`DecalComponent.CreateDynamicMaterialInstance` (`self.LaserDot`)))