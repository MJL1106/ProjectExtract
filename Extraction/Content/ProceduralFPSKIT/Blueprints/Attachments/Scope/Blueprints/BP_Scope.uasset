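; Weapon scope attachment for the FPS kit that switches its lens effect on and off when aiming.
; BeginPlay caches the player character, snaps the glass mesh to the scope's ScopeRendererPoint socket and starts a near-per-frame timer feeding glass location into the scope's dynamic material.
; Aim toggles glass visibility and its bump-offset material, sets the scope radius from the character's spawned item, and passes gradient and sight distance to the lens.
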(event `Timer`
  ;[0 0 0] SCOPE
  (`MaterialInstanceDynamic.SetVectorParameterValue` (`self.ScopeMaterialRef`) "ScopeLocation" (`KismetMathLibrary.Conv_VectorToLinearColor` (`SceneComponent.K2_GetComponentLocation` (`self.ScopeGlassMesh`)))))

(event `self.ReceiveBeginPlay`
  ;[0 0 0] SCOPE
  (bind _asbp_fpcharacter (cast `/Game/ProceduralFPSKIT/Blueprints/BP_FPCharacter` (`GameplayStatics.GetPlayerCharacter` 0)))
  (set `self.As BP First Person Character` _asbp_fpcharacter)
  (`KismetSystemLibrary.K2_SetTimerDelegate` (delegate `Timer`) 0.0001 true)
  (`SceneComponent.K2_AttachToComponent` (`self.ScopeGlassMesh`) (`self.Scope`) "ScopeRendererPoint" "SnapToTarget" "SnapToTarget" "KeepWorld" true)
  (`StaticMeshComponent.SetStaticMesh` (`self.Scope`) (`self.ScopeMesh`)))

(fn `Aim`
  (params (`On/Off` :type Boolean) (GradientParam :type "Float (single-precision)" :default 1000.0) (SightDistance :type "Float (single-precision)" :default 1000.0))
  (bind _scopeglassmesh (`self.ScopeGlassMesh`))
  (bind _scopeglassmesh_2 (`self.ScopeGlassMesh`))
  (bind _on_off (`local.On/Off`))
  (bind _returnvalue (`PrimitiveComponent.GetMaterial` _scopeglassmesh 0))
  (`PrimitiveComponent.SetMaterial` _scopeglassmesh_2 0 (select `bool` _on_off :`false` "/Game/ProceduralFPSKIT/Demo/Materials/M_Glass.M_Glass" :`true` "/Game/ProceduralFPSKIT/Demo/Materials/M_ScopeBumpOffset.M_ScopeBumpOffset" :!type "MaterialInterface Object Reference"))
  (`SceneComponent.SetVisibility` _scopeglassmesh_2 _on_off false)
  (`MaterialInstanceDynamic.SetScalarParameterValue` (`self.ScopeMaterialRef`) "ScopeRadius" (`KismetMathLibrary.SelectFloat` (`/Game/ProceduralFPSKIT/Blueprints/Interactables/BP_Item_Base.ScopeRenderRadius` (`/Game/ProceduralFPSKIT/Blueprints/BP_FPCharacter.SpawnedItem` (`self.As BP First Person Character`))) 0.0 (`local.On/Off`)))
  (if (== _returnvalue "/Game/ProceduralFPSKIT/Demo/Materials/M_ScopeBumpOffset.M_ScopeBumpOffset")
    (bind _returnvalue_2 (`PrimitiveComponent.CreateDynamicMaterialInstance` _scopeglassmesh 0 _returnvalue "None"))
    (`MaterialInstanceDynamic.SetScalarParameterValue` _returnvalue_2 "GradientParam" GradientParam)
    (`MaterialInstanceDynamic.SetScalarParameterValue` _returnvalue_2 "SightDistance" SightDistance)))

(fn `UserConstructionScript`
  (bind _returnvalue (`PrimitiveComponent.CreateDynamicMaterialInstance` (`self.Scope`) 0 null "None"))
  (set `self.ScopeMaterialRef` _returnvalue))