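; Interaction component for the first-person kit that lets the player focus and use interaction areas.
; Each tick a camera line trace finds box or custom-shape areas and toggles their focus.
; TryToInteract branches on interaction type: instant for normal and auto, timer-filled hold, button spam, or spam with timed decay.
; Progress drives a round bar on the target's widget, and completion sends an interact interface message to the area's parent actor.
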(event `Stop`
  (bind _focusedinteractionarea (`self.FocusedInteractionArea`))
  ;[0 0 0] Spam With Timer
  ;;[0 0 0] Stop Interaction
  (`/Engine/EditorBlueprintResources/StandardMacros.IsValid` _focusedinteractionarea
    (:`Is Valid`
      (bind _ref (message `/Game/ProceduralFPSKIT/Blueprints/Interfaces/INT_Interaction.Interaction_WidgetRef` (`Actor.GetParentActor` _focusedinteractionarea)))
      (`/Engine/EditorBlueprintResources/StandardMacros.IsValid` _ref
        (:`Is Valid`
          (bind _asui_interaction (cast `/Game/ProceduralFPSKIT/Blueprints/Widgets/UI_Interaction` (`WidgetComponent.GetWidget` _ref)))
          (set `self.CurrentInteractionWidgetRef` _asui_interaction)
          (`/Game/ProceduralFPSKIT/Blueprints/Widgets/UI_RoundBar.SetPercent` (`/Game/ProceduralFPSKIT/Blueprints/Widgets/UI_Interaction.WB_RoundBar` (`self.CurrentInteractionWidgetRef`)) 0.0))))
    (:`Is Not Valid`
      _))
  (`KismetSystemLibrary.K2_ClearAndInvalidateTimerHandle` (`self.SpamTimer`))
  (set `self.InteractionProgress` 0.0)
  (set `self.CurrentInteractionWidgetRef` null)
  (set `self.Count` 0.0))

(event `DecreaseCount`
  ;[0 0 0] Spam With Timer
  (bind _output_get (set `self.Count` (`KismetMathLibrary.FClamp` (- (`self.Count`) 0.002) 0.0 1.01)))
  (`/Game/ProceduralFPSKIT/Blueprints/Widgets/UI_RoundBar.SetPercent` (`/Game/ProceduralFPSKIT/Blueprints/Widgets/UI_Interaction.WB_RoundBar` (`self.CurrentInteractionWidgetRef`)) _output_get))

(event `self.ReceiveTick`
  (params (DeltaSeconds :type "Float (single-precision)"))
  (`self.Trace`))

(event `TryToInteract`
  (params (Try :type Boolean))
  (if Try
    (if (`self.IsTracingInteractionArea`)
      (`self.FocusedInteractionArea`
        (:`then`
          (switch `/Game/ProceduralFPSKIT/Blueprints/Enums/ENUM_Interaction` (`/Game/ProceduralFPSKIT/Blueprints/Interactables/Interaction/BP_InteractionArea_Master.InteractionType` (`self.FocusedInteractionArea`))
            (:`NewEnumerator0`
              ;[0 0 0] Normal Pickup
              (`self.Interact` (`self.FocusedInteractionArea`) :!label _label))
            (:`NewEnumerator3`
              (bind _output_get (set `self.Interaction Duration` (`/Game/ProceduralFPSKIT/Blueprints/Interactables/Interaction/BP_InteractionArea_Master.InteractionDuration` (`self.FocusedInteractionArea`))))
              (if (> _output_get 0.0)
                (`self.GetRefs`)
                ;[0 0 0] Hold Button
                (bind _returnvalue (`KismetSystemLibrary.K2_SetTimerDelegate` (delegate `UpdateInteractionProgress`) (`self.UpdateInteractionInterval`) true))
                (set `self.InteractionTimer` _returnvalue)
                (`KismetSystemLibrary.K2_ClearAndInvalidateTimerHandle` (`self.SpamTimer`))
                (else
                  (goto _label))))
            (:`NewEnumerator1`
              ;[0 0 0] Spam
              (`self.GetRefs`)
              (bind _output_get_2 (set `self.Count` (`KismetMathLibrary.FClamp` (+ (`self.Count`) 0.1) 0.0 1.01)))
              (`/Game/ProceduralFPSKIT/Blueprints/Widgets/UI_RoundBar.SetPercent` (`/Game/ProceduralFPSKIT/Blueprints/Widgets/UI_Interaction.WB_RoundBar` (`self.CurrentInteractionWidgetRef`)) _output_get_2)
              (if (>= (`self.Count`) 1.01)
                (`self.Interact` (`self.FocusedInteractionArea`))
                (`self.Stop`)))
            (:`NewEnumerator2`
              ;[0 0 0] Spam With Timer
              (`self.GetRefs`)
              (bind _output_get_3 (set `self.Count` (`KismetMathLibrary.FClamp` (+ (`self.Count`) 0.1) 0.0 1.01)))
              (`/Game/ProceduralFPSKIT/Blueprints/Widgets/UI_RoundBar.SetPercent` (`/Game/ProceduralFPSKIT/Blueprints/Widgets/UI_Interaction.WB_RoundBar` (`self.CurrentInteractionWidgetRef`)) _output_get_3)
              (if (>= (`self.Count`) 1.01)
                (`self.Interact` (`self.FocusedInteractionArea`))
                (`self.Stop`)
                (else
                  (bind _returnvalue_2 (`KismetSystemLibrary.K2_SetTimerDelegate` (delegate `DecreaseCount`) 0.01 true))
                  (set `self.SpamTimer` _returnvalue_2)
                  (`KismetSystemLibrary.K2_ClearAndInvalidateTimerHandle` (`self.InteractionTimer`)))))
            (:`NewEnumerator4`
              (goto _label))))
        (:`else`)))
    (else
      (`self.StopInteraction`))))

(event `Interact`
  (params (InteractionArea :type "Actor Object Reference"))
  (bind _returnvalue (`Actor.GetParentActor` InteractionArea))
  (`/Engine/EditorBlueprintResources/StandardMacros.IsValid` _returnvalue
    (:`Is Valid`
      (message `/Game/ProceduralFPSKIT/Blueprints/Interfaces/INT_Interaction.Interface_Interact` _returnvalue))))

(event `UpdateInteractionProgress`
  ;[0 0 0] Hold Button
  (bind _output_get (set `self.InteractionProgress` (+ (`self.InteractionProgress`) (* (/ 1.0 (`self.Interaction Duration`)) (`self.UpdateInteractionInterval`)))))
  (bind _currentinteractionwidgetref (`self.CurrentInteractionWidgetRef`)
    (:`then`
      (`/Game/ProceduralFPSKIT/Blueprints/Widgets/UI_RoundBar.SetPercent` (`/Game/ProceduralFPSKIT/Blueprints/Widgets/UI_Interaction.WB_RoundBar` _currentinteractionwidgetref) _output_get)
      (if (>= (`self.InteractionProgress`) 1.0)
        (`self.StopInteraction`)
        (`self.Interact` (`self.FocusedInteractionArea`))))
    (:`else`)))

(fn `StopInteraction`
  (bind _currentinteractionwidgetref (`self.CurrentInteractionWidgetRef`))
  (if (> (`self.InteractionProgress`) 0.0)
    (`KismetSystemLibrary.K2_ClearAndInvalidateTimerHandle` (`self.InteractionTimer`))
    (`/Engine/EditorBlueprintResources/StandardMacros.IsValid` _currentinteractionwidgetref
      (:`Is Valid`
        (`/Game/ProceduralFPSKIT/Blueprints/Widgets/UI_RoundBar.SetPercent` (`/Game/ProceduralFPSKIT/Blueprints/Widgets/UI_Interaction.WB_RoundBar` _currentinteractionwidgetref) 0.0)
        (set `self.InteractionProgress` 0.0)
        (set `self.CurrentInteractionWidgetRef` null)))))

(fn `Trace`
  (bind _returnvalue (`GameplayStatics.GetPlayerCameraManager` 0))
  (bind _returnvalue_2 (`Actor.K2_GetActorLocation` _returnvalue))
  (bind (_outhit _returnvalue_3) (`KismetSystemLibrary.LineTraceSingle` _returnvalue_2 (+ _returnvalue_2 (* (`KismetMathLibrary.GetForwardVector` (`Actor.K2_GetActorRotation` _returnvalue)) (`self.TraceLenght`))) "TraceTypeQuery1" false (`|MakeArray` (cast `/Game/ProceduralFPSKIT/Blueprints/BP_FPCharacter` (`GameplayStatics.GetPlayerCharacter` 0) :!pure true) :!type "Actor Object Reference") "None" false))
  (if _returnvalue_3
    (bind (_bblockinghit _binitialoverlap _time _distance _location _impactpoint _normal _impactnormal _physmat _hitactor) (`GameplayStatics.BreakHitResult` _outhit))
    (if (!= (`self.FocusedActor`) _hitactor)
      (set `self.FocusedActor` _hitactor)
      (bind _returnvalue_4 (`GameplayStatics.GetObjectClass` _hitactor))
      (bind _returnvalue_5 (or (== _returnvalue_4 "/Game/ProceduralFPSKIT/Blueprints/Interactables/Interaction/BP_InteractionArea_Box.BP_InteractionArea_Box_C") (== _returnvalue_4 "/Game/ProceduralFPSKIT/Blueprints/Interactables/Interaction/BP_InteractionArea_CustomShape.BP_InteractionArea_CustomShape_C")))
      (`self.TraceInteractionArea` _returnvalue_5)
      (if _returnvalue_5
        (`self.Stop`)))
    (else
      (`self.TraceInteractionArea` false))))

(fn `TraceInteractionArea`
  (params (Trace :type Boolean))
  (bind _focusedinteractionarea (`self.FocusedInteractionArea`))
  (bind _focusedinteractionarea_2 (`self.FocusedInteractionArea`))
  (if Trace
    (if (`self.IsTracingInteractionArea`)
      (`/Engine/EditorBlueprintResources/StandardMacros.IsValid` _focusedinteractionarea
        (:`Is Valid`
          (`/Game/ProceduralFPSKIT/Blueprints/Interactables/Interaction/BP_InteractionArea_Master.ToggleFocus` _focusedinteractionarea false))))
    ;[0 0 0] Focus
    (bind _asbp_interaction_area_master (cast `/Game/ProceduralFPSKIT/Blueprints/Interactables/Interaction/BP_InteractionArea_Master` (`self.FocusedActor`)))
    (bind _output_get (set `self.FocusedInteractionArea` _asbp_interaction_area_master))
    (`/Game/ProceduralFPSKIT/Blueprints/Interactables/Interaction/BP_InteractionArea_Master.ToggleFocus` _output_get true)
    (set `self.IsTracingInteractionArea` true)
    (elif (`self.IsTracingInteractionArea`)
      (set `self.IsTracingInteractionArea` false)
      (`/Engine/EditorBlueprintResources/StandardMacros.IsValid` _focusedinteractionarea_2
        (:`Is Valid`
          (`/Game/ProceduralFPSKIT/Blueprints/Interactables/Interaction/BP_InteractionArea_Master.ToggleFocus` _focusedinteractionarea_2 false)
          (set `self.FocusedActor` null)
          (set `self.FocusedInteractionArea` null)
          (`self.StopInteraction`))))))