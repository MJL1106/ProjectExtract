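; Deprecated actor component that plays turn-in-place montages on its owning Character in the procedural FPS kit.
; TurnInPlace compares actor and aim yaw while grounded, still and uncrouched, choosing a 90 or 180 degree left or right turn.
; PlayTurn blocks re-entry with a Turning flag, and ClearTurnInPlace stops root-motion montages when Force is non-zero.
; Tick is unused, and the turn events show no montage assigned.
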(event `self.ReceiveBeginPlay`
  (bind _ascharacter (cast `Character` (`self.GetOwner`)))
  (bind _output_get (set `self.As Character` _ascharacter))
  (set `self.Mesh` (`Character.Mesh` _output_get))
  (set `self.Character Movement` (`Character.CharacterMovement` _output_get)))

(event `PlayTurn`
  (params (MontageToPlay :type "AnimMontage Object Reference") (PlayRate :type "Float (single-precision)" :default 1.0) (Duration :type "Float (single-precision)"))
  (if (not (`self.Turning`))
    (set `self.Turning` true)
    (`|PlayMontage` (`self.Mesh`) MontageToPlay PlayRate
      (:`then`
        (`KismetSystemLibrary.Delay` Duration))
      (:`OnCompleted`
        _))
    ;[1 1 1] Comment
    (set `self.Turning` false)))

(event `ClearMotion`
  (bind _as_character (`self.As Character`))
  (if (`Character.IsPlayingRootMotion` (`self.As Character`))
    (`Character.StopAnimMontage` _as_character (`Character.GetCurrentMontage` _as_character))))

(event `TurnRight90`
  (`self.PlayTurn` null 1.5 0.5))

(event `TurnLeft90`
  (`self.PlayTurn` null 1.5 0.5))

(event `ClearTurnInPlace`
  (params (Force :type "Float (double-precision)"))
  (if (!= Force 0.0)
    (`self.ClearMotion`)))

(event `TurnRight180`
  (`self.PlayTurn` null 1.7 0.6))

(event `TurnLeft180`
  (`self.PlayTurn` null 1.7 0.6))

(fn `TurnInPlace`
  (bind _character_movement (`self.Character Movement`))
  (bind _as_character (`self.As Character`))
  (bind (_returnvalue_roll _returnvalue_pitch _returnvalue_yaw) (`KismetMathLibrary.BreakRotator` (`KismetMathLibrary.NormalizedDeltaRotator` (`Actor.K2_GetActorRotation` _as_character) (`Pawn.GetBaseAimRotation` _as_character))))
  (bind _returnvalue (* _returnvalue_yaw -1.0))
  (if (and (not (`NavMovementComponent.IsFalling` _character_movement)) (not (> (`KismetMathLibrary.VSizeXY` (`MovementComponent.Velocity` _character_movement)) 0.0)) (not (`NavMovementComponent.IsCrouching` _character_movement)))
    (if (or (> _returnvalue 45.0) (< _returnvalue -45.0))
      (if (> _returnvalue 135.0)
        (`self.TurnRight180`)
        (elif (< _returnvalue -135.0)
          (`self.TurnLeft180`)
          (elif (> _returnvalue 45.0)
            (`self.TurnRight90`)
            (elif (< _returnvalue -45.0)
              (`self.TurnLeft90`))))))))