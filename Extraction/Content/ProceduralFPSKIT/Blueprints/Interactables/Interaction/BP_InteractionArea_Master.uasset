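; Master interaction area that relays focus and overlap-triggered interaction to its parent actor through interface messages.
; An optional CheckCollision box limits gaining focus to when a BP_FPCharacter is inside it, while losing focus always passes through.
; One InteractionType also sends an interact message as soon as the character enters the box.
; The construction script sizes, positions and shows the box when either mode needs it, otherwise hiding it.
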(event `ToggleFocus`
  (params (Focused :type Boolean))
  (set `self.Focused` Focused)
  (if (`self.CheckCollisionBoxPermission`)
    (if (`self.CanFocus`)
      (message `/Game/ProceduralFPSKIT/Blueprints/Interfaces/INT_Interaction.Interface_ToggleFocus` (`self.GetParentActor`) (`self.Focused`) :!label _label)
      (elif (== (`self.Focused`) false)
        (goto _label)))
    (else
      (goto _label))))

(event `self.CheckCollision.OnComponentBeginOverlap`
  (params (OverlappedComponent :type "PrimitiveComponent Object Reference") (OtherActor :type "Actor Object Reference") (OtherComp :type "PrimitiveComponent Object Reference") (OtherBodyIndex :type Integer) (bFromSweep :type Boolean) (SweepResult :type "HitResult Structure (by ref)"))
  (cast `/Game/ProceduralFPSKIT/Blueprints/BP_FPCharacter` OtherActor)
  (set `self.CanFocus` true)
  (if (`|EnumEquality` (`self.InteractionType`) "NewEnumerator4")
    (message `/Game/ProceduralFPSKIT/Blueprints/Interfaces/INT_Interaction.Interface_Interact` (`self.GetParentActor`))))

(event `self.CheckCollision.OnComponentEndOverlap`
  (params (OverlappedComponent :type "PrimitiveComponent Object Reference") (OtherActor :type "Actor Object Reference") (OtherComp :type "PrimitiveComponent Object Reference") (OtherBodyIndex :type Integer))
  (cast `/Game/ProceduralFPSKIT/Blueprints/BP_FPCharacter` OtherActor)
  (set `self.CanFocus` false))

(fn `UserConstructionScript`
  (bind _checkcollision (`self.CheckCollision`))
  (bind _checkcollision_2 (`self.CheckCollision`))
  (if (or (`self.CheckCollisionBoxPermission`) (`|EnumEquality` (`self.InteractionType`) "NewEnumerator4"))
    (`SceneComponent.SetVisibility` _checkcollision_2 true false)
    (`BoxComponent.SetBoxExtent` _checkcollision (`self.CheckCollisionBoxSize`) true)
    (`SceneComponent.K2_SetRelativeLocation` _checkcollision (`self.CheckCollisionLocation`) false true)
    (else
      (`SceneComponent.SetVisibility` _checkcollision_2 false false))))