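; BP_GranadeProjectile is a thrown or launched grenade that explodes on a two-second fuse started at BeginPlay.
; On detonation it spawns the explosion particles, deals full radial damage blocked by the Camera channel, then a tick later fires a RadialForce impulse, plays the sound and destroys itself.
; While bouncing, hits push physics-simulating components along the grenade's velocity and play a bounce sound, capped by a DoN.
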(event `self.ReceiveBeginPlay`
  (bind _radialforce (`self.RadialForce`))
  (bind _returnvalue (`SceneComponent.K2_GetComponentLocation` (`self.SkeletalMesh`)))
  ;[0 0 0] BOMB EXPLOSION
  (`KismetSystemLibrary.Delay` 2.0)
  (`GameplayStatics.SpawnEmitterAtLocation` "/Game/ProceduralFPSKIT/ParticleEffects/P_Grenade_Explosion.P_Grenade_Explosion" _returnvalue (struct) (2.0 2.0 2.0) true "AutoRelease")
  (`self.KillEnemies`)
  (`KismetSystemLibrary.DelayUntilNextTick`)
  (set `RadialForceComponent.Radius` 600.0 _radialforce)
  (set `RadialForceComponent.ImpulseStrength` 450.0 _radialforce)
  (`RadialForceComponent.FireImpulse` _radialforce)
  (`GameplayStatics.PlaySoundAtLocation` "/Game/ProceduralFPSKIT/Audio/Character/Grenade_Explosion_Cue.Grenade_Explosion_Cue" _returnvalue (struct) 2.0 1.0 0.0 "/Game/ProceduralFPSKIT/Audio/Attenuation/Explosion_att.Explosion_att" null null null)
  (`self.K2_DestroyActor`))

(event `self.ReceiveHit`
  (params (MyComp :type "PrimitiveComponent Object Reference") (Other :type "Actor Object Reference") (OtherComp :type "PrimitiveComponent Object Reference") (bSelfMoved :type Boolean) (HitLocation :type "Vector Structure") (HitNormal :type "Vector Structure") (NormalImpulse :type "Vector Structure") (Hit :type "HitResult Structure (by ref)"))
  (bind _returnvalue (`self.K2_GetActorLocation`))
  ;[0 0 0] ADD IMPULSE TO OBJECTS WE HIT AND HIT SOUND
  (if (`SceneComponent.IsSimulatingPhysics` OtherComp "None")
    (`PrimitiveComponent.AddImpulseAtLocation` OtherComp (* (`self.GetVelocity`) 1.5) _returnvalue "None"))
  (`/Engine/EditorBlueprintResources/StandardMacros.Do N` 7
    (:`Exit`
      (`GameplayStatics.PlaySoundAtLocation` "/Game/ProceduralFPSKIT/Audio/Character/GrenadeLauncher_Bounce_Cue.GrenadeLauncher_Bounce_Cue" _returnvalue (struct) 0.5 1.0 0.0 "/Game/ProceduralFPSKIT/Audio/Attenuation/ProjectileImpact_att.ProjectileImpact_att" null null null))))

(event `KillEnemies`
  ;[0 0 0] KILL ENEMIES ON THE RADIUS
  (`GameplayStatics.ApplyRadialDamage` 1000.0 (`SceneComponent.K2_GetComponentLocation` (`self.CollisionComponent`)) 500.0 null (`|MakeArray` self :!type "Actor Object Reference") self null true "ECC_Camera"))

(fn `UserConstructionScript`)