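; BP_ExtractionCharacter is a character Blueprint that wires a HealthComponent to debug feedback for damage and death.
; On BeginPlay it binds handlers to the component's health-changed and death events, each of which only prints a message.
; Pressing H applies a fixed amount of damage through the component as a test input.
; Tick, overlap and construction logic are empty.
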(event `self.ReceiveBeginPlay`
  (add `HealthComponent.OnHealthChanged` (`self.HealthComponent`) (`|CreateDelegate` :!event `OnHealthChangedEvent`))
  (add `HealthComponent.OnDeath` (`self.HealthComponent`) (`|CreateDelegate` :!event `OnDeathEvent`)))

(event `OnHealthChangedEvent`
  (params (CurrentHealth :type "Float (double-precision)") (MaxHealth :type "Float (double-precision)"))
  (`KismetSystemLibrary.PrintString` "Health Changed!"))

(event `OnDeathEvent`
  (`KismetSystemLibrary.PrintString` "DEAD!" true true (struct :`R` 1.0 :`A` 1.0) 5.0))

(event `Key|H`
  (params (Key :type "Key Structure"))
  (:`Pressed`
    (`HealthComponent.TakeDamage` (`self.HealthComponent`) 20.0)))

(fn `UserConstructionScript`)